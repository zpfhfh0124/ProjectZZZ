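; Player character Blueprint with camera-relative movement, look rotation and a melee-style attack.
; BeginPlay spawns BP_AnbyWeapon and attaches it to the right-hand socket.
; Enhanced Input drives movement and run/walk flags, halving Speed while walking, as Tick feeds look input into controller and actor rotation.
; Left click plays the montage indexed by AttackState, which resets to its first value; right click is a stub.
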(event Input|EnhancedActionEvents|EnhancedInputActionIA_LMB
  (params (ActionValue :type Boolean) (ElapsedSeconds :type Float%20%28double-precision%29) (TriggeredSeconds :type Float%20%28double-precision%29) (InputAction :type Input%20Action%20Object%20Reference :default "/Game/IA_LMB.IA_LMB"))
  ;[0.2599 0.7565 0.5531 0.5] Attack
  (CallFunction|Attack))

(event Input|EnhancedActionEvents|EnhancedInputActionIA_Controll
  (params (ActionValue :type Boolean) (ElapsedSeconds :type Float%20%28double-precision%29) (TriggeredSeconds :type Float%20%28double-precision%29) (InputAction :type Input%20Action%20Object%20Reference :default "/Game/IA_Controll.IA_Controll"))
  ;[0.15 0.03749 0.1259 0.5] Movement
  ;;[0.1467 0.15 0.03591 0.5] Run/Walk
  (:Started
    (Variables|Default|SetIsWalk true)
    (Variables|Default|SetSpeed (/ (Variables|Default|GetSpeed) 2.0)))
  (:Completed
    (Variables|Default|SetIsWalk false)
    (Variables|Default|SetSpeed (* (Variables|Default|GetSpeed) 2.0))))

(event Input|EnhancedActionEvents|EnhancedInputActionIA_Vertical
  (params (ActionValue :type Float%20%28double-precision%29) (ElapsedSeconds :type Float%20%28double-precision%29) (TriggeredSeconds :type Float%20%28double-precision%29) (InputAction :type Input%20Action%20Object%20Reference :default "/Game/Doeun/Inputs/IA_Vertical.IA_Vertical"))
  (:Triggered
    ;[0.15 0.03749 0.1259 0.5] Movement
    (Pawn|Input|AddMovementInput (Math|Vector|GetForwardVector (Variables|Default|GetCamera)) ActionValue false)
    (Variables|Default|SetIsRun true))
  (:Completed
    (Variables|Default|SetIsRun false)))

(event Input|EnhancedActionEvents|EnhancedInputActionIA_Horizontal
  (params (ActionValue :type Float%20%28double-precision%29) (ElapsedSeconds :type Float%20%28double-precision%29) (TriggeredSeconds :type Float%20%28double-precision%29) (InputAction :type Input%20Action%20Object%20Reference :default "/Game/Doeun/Inputs/IA_Horizontal.IA_Horizontal"))
  (:Triggered
    ;[0.15 0.03749 0.1259 0.5] Movement
    (Pawn|Input|AddMovementInput (Math|Vector|GetRightVector (Variables|Default|GetCamera)) ActionValue false)
    (Variables|Default|SetIsRun true))
  (:Completed
    (Variables|Default|SetIsRun false)))

(event Input|EnhancedActionEvents|EnhancedInputActionIA_RMB
  (params (ActionValue :type Boolean) (ElapsedSeconds :type Float%20%28double-precision%29) (TriggeredSeconds :type Float%20%28double-precision%29) (InputAction :type Input%20Action%20Object%20Reference :default "/Game/IA_RMB.IA_RMB"))
  (if true
    _))

(event EventBeginPlay
  ;[0.15 0.1269 0.03315 0.5] Weapon Equip
  (bind _output_get (Variables|Default|SetWeaponSocketName "RightHandSocket"))
  (bind _returnvalue (Game|SpawnActorfromClass "/Game/BP_AnbyWeapon.BP_AnbyWeapon_C" (Transformation|GetSocketTransform (Variables|Character|GetMesh) _output_get "RTS_World") "Undefined" "MultiplyWithRoot" 0 0))
  (Transformation|AttachComponentToComponent _returnvalue (Variables|Character|GetMesh) (Variables|Default|GetWeaponSocketName) "SnapToTarget" "SnapToTarget" "SnapToTarget" true)
  (Variables|Default|SetAttackState "NewEnumerator0"))

(event Collision|EventActorBeginOverlap
  (params (OtherActor :type Actor%20Object%20Reference)))

(event EventTick
  (params (DeltaSeconds :type Float%20%28single-precision%29))
  (bind _returnvalue (Input|EnhancedActionValues|GetIA_PlayerRotation))
  (Utilities|FlowControl|Sequence
    (:then_0
      ;[0.15 0.04196 0.04482 0.5] Rotation (Camera)
      (CallFunction|SetRotation DeltaSeconds (.x _returnvalue) (.x _returnvalue) (.y _returnvalue) (.y _returnvalue)))))

(fn ConstructionScript)

(fn SetRotation
  (params (InputPin :type Float%20%28single-precision%29) (InputPin2 :type Float%20%28double-precision%29) (Val :type Float%20%28single-precision%29) (Y :type Float%20%28double-precision%29) (Val2 :type Float%20%28single-precision%29))
  (bind _returnvalue (Transformation|GetActorRotation))
  (bind _returnvalue_2 (Math|Vector|MakeVector 0.0 Y InputPin2))
  (bind _returnvalue_3 (Math|Vector|Normalize _returnvalue_2))
  (bind _returnvalue_4 (* InputPin _returnvalue_3))
  (bind _returnvalue_5 (+ (Math|Vector|MakeVector 0.0 (.pitch _returnvalue) (.yaw _returnvalue)) _returnvalue_4))
  (Pawn|Input|AddControllerPitchInput Val2)
  (Pawn|Input|AddControllerYawInput Val)
  (Transformation|SetActorRotation (Math|Rotator|MakeRotator (.roll _returnvalue) (.y _returnvalue_5) (.z _returnvalue_5))))

(fn Attack
  (Animation|PlayAnimMontage (Utilities|Array|Get(acopy) (Variables|Default|GetAttackAnimMontageList) (Math|Conversions|ToInteger(Byte) (Variables|Default|GetAttackState))) 1.0 "None")
  (Variables|Default|SetAttackState "NewEnumerator0"))
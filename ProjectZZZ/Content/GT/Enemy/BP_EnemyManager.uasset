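; BP_EnemyManager is a placed spawner that creates a one-time group of Phobos enemies when the player comes near.
; BeginPlay caches the player character, and Tick checks its 2D distance to the manager until spawning happens, logging an error if no player exists.
; SpawnEnemy spawns MaxSpawn BP_EnemyPhobos at random reachable navmesh points within SpawnRadius, turns each toward the player, then sets IsSpawned.
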(event EventBeginPlay
  (bind _returnvalue (Actor|GetActorOfClass "/Game/BP_PlayerCharacter.BP_PlayerCharacter_C"))
  (Variables|Default|SetPlayer _returnvalue))

(event Collision|EventActorBeginOverlap
  (params (OtherActor :type Actor%20Object%20Reference)))

(event EventTick
  (params (DeltaSeconds :type Float%20%28single-precision%29))
  ;[0.07135 0.15 0.07778 0.5] 몬스터 생성
  (Utilities|IsValid (Variables|Default|GetPlayer)
    (:Is%20Valid
      (if (not (Variables|Default|GetIsSpawned))
        (CallFunction|SpawnEnemy (Variables|Default|GetPlayer))))
    (:Is%20Not%20Valid
      (Class|AutomationBlueprintFunctionLibrary|AddExpectedLogError "플레이어를 찾지 못했다."))))

(fn ConstructionScript)

(fn SpawnEnemy
  (params (self2 :type Actor%20Object%20Reference))
  (bind _returnvalue (Transformation|GetActorLocation))
  (bind _returnvalue_2 (Transformation|GetActorLocation self2))
  (bind _returnvalue_3 (Math|Vector|Distance2D(Vector) _returnvalue_2 _returnvalue))
  (Development|PrintString (Utilities|String|ToString(Float) _returnvalue_3))
  (if (<= _returnvalue_3 (Variables|Default|GetDistance))
    (for _index (range 1 (Variables|Default|GetMaxSpawn))
      (bind _returnvalue_4 (Game|SpawnActorfromClass "/Game/GT/Enemy/BP_EnemyPhobos.BP_EnemyPhobos_C" (Math|Transform|MakeTransform (.RandomLocation (AI|Navigation|GetRandomReachablePointinRadius _returnvalue (Variables|Default|GetSpawnRadius) 0 0)) "0, 0, 0" "1.000000,1.000000,1.000000") "Undefined" "MultiplyWithRoot" 0 0))
      ;[0.0471 0.15 0.04826 0.5] 스폰 이후 플레이어 방향으로 설정
      (Transformation|SetActorRotation _returnvalue_4 (Math|Conversions|RotationFromXVector (- (Transformation|GetActorLocation (Variables|Default|GetPlayer)) (Transformation|GetActorLocation _returnvalue_4)))))
    (Variables|Default|SetIsSpawned true)))
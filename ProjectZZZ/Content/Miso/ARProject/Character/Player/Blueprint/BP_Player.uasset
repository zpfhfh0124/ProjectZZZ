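; BP_Player is the player pawn Blueprint, handling movement, run and look input.
; BeginPlay adds an Enhanced Input mapping context, whose actions set IsRun and drive controller yaw and pitch.
; Legacy MoveForward and MoveRight axes act as a hardcoded movement fallback along actor vectors.
; The Enhanced Move action, marked as malfunctioning, only applies movement while running, doubling sideways input and zeroing forward; otherwise it just stores values.
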(event Input|EnhancedActionEvents|EnhancedInputActionMS_IA_Move
  (params (ActionValue :type Vector%202D%20Structure) (ElapsedSeconds :type Float%20%28double-precision%29) (TriggeredSeconds :type Float%20%28double-precision%29) (InputAction :type Input%20Action%20Object%20Reference :default "/Game/Miso/ARProject/Controller/InputAction/MS_IA_Move.MS_IA_Move"))
  (bind _returnvalue (Pawn|GetControlRotation :!class /Script/Engine.Pawn))
  ;[0.15 0.15 0.15 0.5] Move <- 제대로 동작 안함
  (:Triggered
    (if (Variables|Move|GetIs%20Run)
      (Variables|Move|SetSideInput (* (.x ActionValue) 2.0))
      (Variables|Move|SetForwardInput (* 0.0 (.y ActionValue)))
      (Pawn|Input|AddMovementInput (Math|Vector|GetRightVector _returnvalue) (Variables|Move|GetSideInput) false)
      (Pawn|Input|AddMovementInput (Math|Vector|GetForwardVector _returnvalue) (Variables|Move|GetForwardInput) false)
      (else
        (Variables|Move|SetSideInput (.x ActionValue))
        (Variables|Move|SetForwardInput (.y ActionValue)))))
  (:Canceled
    (Variables|Move|SetSideInput 0.0)
    (Variables|Move|SetForwardInput 0.0)))

(event Input|EnhancedActionEvents|EnhancedInputActionMS_IA_Run
  (params (ActionValue :type Boolean) (ElapsedSeconds :type Float%20%28double-precision%29) (TriggeredSeconds :type Float%20%28double-precision%29) (InputAction :type Input%20Action%20Object%20Reference :default "/Game/Miso/ARProject/Controller/InputAction/MS_IA_Run.MS_IA_Run"))
  ;[0.15 0.15 0.15 0.5] Run
  (:Triggered
    (Variables|Move|SetIs%20Run ActionValue :!label _label))
  (:Completed
    (goto _label)))

(event Input|EnhancedActionEvents|EnhancedInputActionMS_IA_Look
  (params (ActionValue :type Vector%202D%20Structure) (ElapsedSeconds :type Float%20%28double-precision%29) (TriggeredSeconds :type Float%20%28double-precision%29) (InputAction :type Input%20Action%20Object%20Reference :default "/Game/Miso/ARProject/Controller/InputAction/MS_IA_Look.MS_IA_Look"))
  ;[0.15 0.15 0.15 0.5] Look
  (Pawn|Input|AddControllerYawInput (.x ActionValue))
  (Pawn|Input|AddControllerPitchInput (.y ActionValue)))

(event EventBeginPlay
  ;[0.15 0.15 0.15 0.5] InputMapping
  (bind _asplayer_controller (Utilities|Casting|CastToPlayerController (Pawn|GetController)))
  (Utilities|IsValid _asplayer_controller
    (:Is%20Valid
      (Input|AddMappingContext (PlayerController|LocalPlayerSubsystems|GetEnhancedInputLocalPlayerSubsystem _asplayer_controller) "/Game/Miso/ARProject/Controller/MS_IMC_PlayerController.MS_IMC_PlayerController" 0 "(bIgnoreAllPressedKeysUntilRelease=True,bForceImmediately=False,bNotifyUserSettings=False)"))))

(event Input|AxisEvents|InputAxisMoveForward
  (params (AxisValue :type Float%20%28single-precision%29))
  ;[0.15 0.15 0.15 0.5] Move - 하드코딩
  (bind _output_get (Variables|Move|SetForwardInput AxisValue))
  (Pawn|Input|AddMovementInput (Transformation|GetActorForwardVector (Components|GetOwner)) _output_get false))

(event Input|AxisEvents|InputAxisMoveRight
  (params (AxisValue :type Float%20%28single-precision%29))
  ;[0.15 0.15 0.15 0.5] Move - 하드코딩
  (bind _output_get (Variables|Move|SetSideInput AxisValue))
  (Pawn|Input|AddMovementInput (Transformation|GetActorRightVector (Components|GetOwner)) _output_get false))

(fn ConstructionScript)
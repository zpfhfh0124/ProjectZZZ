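; BP_EnemyHati is an enemy character that pursues the player and loses HP when hit by Anby's weapon.
; BeginPlay caches its HP bar widget and starts a single AIMoveTo toward the player, stopping at attack range.
; Weapon overlap feeds SetDamage, which clamps HP and flags death at zero; negative damage heals.
; Attack and hit-react functions play Cyclops montages and set state flags, while manual view-cone chase logic sits disconnected.
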(event Custom|ChasePlayer_Event)

(event EventBeginPlay
  (Utilities|FlowControl|Sequence
    (:then_0
      (bind _returnvalue (Actor|GetActorOfClass "/Game/BP_PlayerCharacter.BP_PlayerCharacter_C"))
      (bind _output_get (Variables|Default|SetTargetPlayer _returnvalue))
      ;[0.15 0.15 0.15 0.5] 플레이어 AI 적용
      (AI|AIMoveTo self "0, 0, 0" _output_get (Variables|Default|GetAttackDistance) false))
    (:then_1
      ;[0.15 0.15 0.15 0.5] 위젯 변수 할당
      (bind _aswbp_enemy_hpbar (Utilities|Casting|CastToWBP_EnemyHPBar (UserInterface|GetWidget (Variables|Default|GetWidgetHP))))
      (Variables|Default|SetWidgetHPBar _aswbp_enemy_hpbar))))

(event Collision|EventActorBeginOverlap
  (params (OtherActor :type Actor%20Object%20Reference))
  (bind _asbp_anby_weapon (Utilities|Casting|CastToBP_AnbyWeapon OtherActor)
    (:then
      (CallFunction|SetDamage (Variables|/Game/BP_AnbyWeapon.BP_AnbyWeapon_C|GetFinDamage _asbp_anby_weapon)))
    (:CastFailed
      (Class|VisualLoggerKismetLibrary|LogText 0 "오버랩 되었지만 Anby Weapon은 아니다." "VisLogBP"))))

(event EventTick
  (params (DeltaSeconds :type Float%20%28single-precision%29))
  (Utilities|FlowControl|Sequence))

(event Collision|EventActorEndOverlap
  (params (OtherActor :type Actor%20Object%20Reference))
  (CallFunction|EndAttack))

(fn ConstructionScript)

(fn StartAttack
  (Animation|PlayAnimMontage "/Game/Resources/Monsters/Monster_Cyclops_Model/Cyclops_Attack_Montage.Cyclops_Attack_Montage" 1.0 "None")
  (Variables|Default|SetIsAttack true))

(fn EndAttack
  (Variables|Default|SetIsAttack false))

(fn StartHitReact
  (Animation|PlayAnimMontage "/Game/Resources/Monsters/Monster_Cyclops_Model/Cyclops_Hit_Montage.Cyclops_Hit_Montage" 1.0 "None")
  (Variables|Default|SetIsHit true))

(fn EndHitReact
  (Variables|Default|SetIsHit false))

(fn Die
  (Variables|Default|SetIsDie true))

(fn SetDamage
  (params (Damage :type Integer))
  (bind _output_get (Variables|Default|SetCurrHP (Math|Integer|Clamp(Integer) (- (Variables|Default|GetCurrHP) Damage) 0 (Variables|Default|GetMaxHP))))
  (if (<= _output_get 0)
    (CallFunction|Die)))
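; BP_EnemyA is an enemy that chases the player and flags when it should attack.
; BeginPlay caches the BP_PlayerCharacter, and ChasePlayer_Event runs AI MoveTo toward it, using the attack distance as acceptance radius.
; The move's success or failure feeds Attack, which only sets IsAttack.
; Tick is empty; older view-angle chase and look-at logic remains disconnected and never runs.
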(event Custom|ChasePlayer_Event
  ;[0.15 0.15 0.15 0.5] 플레이어 추격 및 공격
  (AI|AIMoveTo self "0, 0, 0" (stale EventBeginPlay _output_get) (Variables|Default|GetAttackDistance) false
    (:OnSuccess
      (CallFunction|Attack true))
    (:OnFail
      (CallFunction|Attack false))))

(event EventBeginPlay
  (bind _returnvalue (Actor|GetActorOfClass "/Game/BP_PlayerCharacter.BP_PlayerCharacter_C"))
  (bind _output_get (Variables|Default|SetPlayer _returnvalue)))

(event Collision|EventActorBeginOverlap
  (params (OtherActor :type Actor%20Object%20Reference)))

(event EventTick
  (params (DeltaSeconds :type Float%20%28single-precision%29)))

(fn ConstructionScript)

(fn Attack
  (params (IsAttack :type Boolean))
  (Variables|Default|SetIsAttack IsAttack))
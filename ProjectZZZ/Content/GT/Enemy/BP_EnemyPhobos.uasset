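; BP_EnemyPhobos is an enemy that chases the player inside its view angle and flags when it is close enough to attack.
; BeginPlay caches the player; Tick tests the angle using a dot product with the unnormalized offset, then moves straight toward them without sweep.
; While chasing, 2D distance sets IsAttack; the attack itself is absent here.
; The look-at rotation logic is disconnected, and a missing player logs an error.
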(event EventBeginPlay
  (bind _returnvalue (Actor|GetActorOfClass "/Game/BP_PlayerCharacter.BP_PlayerCharacter_C"))
  (Variables|Default|SetPlayer _returnvalue))

(event Collision|EventActorBeginOverlap
  (params (OtherActor :type Actor%20Object%20Reference)))

(event EventTick
  (params (DeltaSeconds :type Float%20%28single-precision%29))
  (bind _returnvalue (Transformation|GetActorLocation))
  (bind _player (Variables|Default|GetPlayer))
  (bind _returnvalue_2 (Transformation|GetActorLocation _player))
  (bind _returnvalue_3 (- _returnvalue_2 _returnvalue))
  (Utilities|FlowControl|Sequence
    (:then_0
      ;[0.15 0.05159 0.1376 0.5] 시야각 안으로 들어오면 플레이어 추격
      (Utilities|IsValid (Variables|Default|GetPlayer)
        (:Is%20Valid
          (bind _output_get (Variables|Default|SetIsMove (<= (Class|KismetMathLibrary|DegAcos (Math|Vector|DotProduct (Transformation|GetActorForwardVector) _returnvalue_3)) (/ (Variables|Default|GetViewAngle) 2))))
          (if _output_get
            (Transformation|SetActorLocation (+ (Transformation|GetActorLocation) (* DeltaSeconds (* (Variables|Default|GetSpeed) (Math|Vector|Normalize _returnvalue_3)))) false false)
            ;;[0.04385 0.07444 0.15 0.5] 근접해지면 공격 시전
            (if (<= (Math|Vector|Distance2D(Vector) (Transformation|GetActorLocation) (Transformation|GetActorLocation (Variables|Default|GetPlayer))) (Variables|Default|GetAttackDistance))
              (Variables|Default|SetIsAttack true)
              (else
                (Variables|Default|SetIsAttack false)))))
        (:Is%20Not%20Valid
          (Class|AutomationBlueprintFunctionLibrary|AddExpectedLogError "생성된 적이 플레이어를 찾을 수 없음"))))
    (:then_1)))

(fn ConstructionScript)